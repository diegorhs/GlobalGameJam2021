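; BP_Player is a player character that moves by dashing along the camera's view direction.
; Turn and LookUp axes rotate the controller, and the DashForward and DashBack actions launch the character along or against the control rotation's forward vector, replacing current velocity.
; Every tick, an additive launch opposes the normalized velocity by StopForce, acting as a constant brake that is not scaled by delta time.
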(event EventTick
  (params (DeltaSeconds :type Float%20%28single-precision%29))
  (Character|LaunchCharacter (* (* (Math|Vector|Normalize (Variables|/Script/Engine.MovementComponent|GetVelocity (Variables|Character|GetCharacterMovement))) (Variables|Default|GetStopForce)) -1) false false))

(event Input|ActionEvents|InputActionDashForward
  (params (Key :type Key%20Structure :default "None"))
  (:Pressed
    (Character|LaunchCharacter (* (Math|Vector|GetForwardVector (Pawn|GetControlRotation :!class /Script/Engine.Pawn)) (Variables|Default|GetMovementForce)) true true)))

(event Input|ActionEvents|InputActionDashBack
  (params (Key :type Key%20Structure :default "None"))
  (:Pressed
    (Character|LaunchCharacter (* (* (Math|Vector|GetForwardVector (Pawn|GetControlRotation :!class /Script/Engine.Pawn)) (Variables|Default|GetMovementForce)) -1) true true)))

(event Input|AxisEvents|InputAxisTurn
  (params (AxisValue :type Float%20%28single-precision%29))
  (Pawn|Input|AddControllerYawInput AxisValue))

(event Input|AxisEvents|InputAxisLookUp
  (params (AxisValue :type Float%20%28single-precision%29))
  (Pawn|Input|AddControllerPitchInput AxisValue))

(fn ConstructionScript)