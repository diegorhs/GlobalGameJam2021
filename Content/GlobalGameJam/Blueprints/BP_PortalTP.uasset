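; BP_PortalTP drives the see-through view between two linked portals by positioning Portal2's scene capture relative to the player camera.
; Every tick, Portal1Update offsets the camera location by the vector from Portal2 to Portal1 and applies it to the capture with the camera's rotation.
; The mapping is translation-only, ignoring portal orientation, and updates one direction without any teleport logic.
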(event EventTick
  (params (DeltaSeconds :type Float%20%28single-precision%29))
  (CallFunction|Portal1Update))

(fn ConstructionScript)

(fn Portal1Update
  (bind _returnvalue (Game|GetPlayerCameraManager 0))
  (bind _transformcomponent (Variables|/Script/Engine.PlayerCameraManager|GetTransformComponent _returnvalue))
  (Transformation|SetWorldLocationAndRotation (Variables|/Game/GlobalGameJam/Blueprints/BP_Portal2.BP_Portal2_C|GetSceneCaptureComponent2D (Variables|Default|GetPortal%202)) (+ (- (Transformation|GetWorldLocation (Variables|/Script/Engine.Actor|GetRootComponent (Variables|Default|GetPortal%201))) (Transformation|GetWorldLocation (Variables|/Script/Engine.Actor|GetRootComponent (Variables|Default|GetPortal%202)))) (Transformation|GetWorldLocation _transformcomponent)) (Transformation|GetWorldRotation _transformcomponent) false false))