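; Player character for a Global Game Jam game that moves by camera-directed dashes, forward or back.
; BeginPlay creates the HUD, starts audio and randomizes mesh, animation and constellation FX.
; Dashes launch faster when GetCanBoost passes, charging a beat meter that drains by timeline once full; Tick decelerates them, and non-portal hits stop them.
; Pause or a depleted StarCount pauses with the victory widget, while Z toggles mouse-sensitivity UI.
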(event OnComponentHit(CapsuleComponent)
  (params (HitComponent :type Primitive%20Component%20Object%20Reference) (OtherActor :type Actor%20Object%20Reference) (OtherComp :type Primitive%20Component%20Object%20Reference) (NormalImpulse :type Vector :default "0, 0, 0") (Hit :type Hit%20Result%20Structure%20%28by%20ref%29))
  ;[1 1 1] Si se choca, se para
  (Utilities|Casting|CastToBP_PortalDoor OtherActor
    (:CastFailed
      (Variables|/Script/Engine.MovementComponent|SetVelocity (Variables|Character|GetCharacterMovement) "0, 0, 0")
      (Variables|Default|SetDashActivated false))))

(event EventTick
  (params (DeltaSeconds :type Float%20%28single-precision%29))
  ;[1 1 1] Reduce Velocity
  (if (> (Variables|Default|GetStarCount) 0.0)
    (if (Math|Vector|Equal(Vector) (Variables|/Script/Engine.MovementComponent|GetVelocity (Variables|Character|GetCharacterMovement)) "0, 0, 0" 1e+01)
      (Variables|/Script/Engine.MovementComponent|SetVelocity (Variables|Character|GetCharacterMovement) "0, 0, 0")
      (Variables|Default|SetDashActivated false)
      (elif (> (Variables|Default|GetLastSpeedValue) 0.0)
        (Variables|/Script/Engine.MovementComponent|SetVelocity (Variables|Character|GetCharacterMovement) (- (Variables|/Script/Engine.MovementComponent|GetVelocity (Variables|Character|GetCharacterMovement)) (* (Variables|Default|GetLastDirection) (Variables|Default|GetReduceVelocity))))
        (else
          (Variables|/Script/Engine.MovementComponent|SetVelocity (Variables|Character|GetCharacterMovement) (+ (Variables|/Script/Engine.MovementComponent|GetVelocity (Variables|Character|GetCharacterMovement)) (* (Variables|Default|GetLastDirection) (Variables|Default|GetReduceVelocity)))))))
    (else
      (bind _returnvalue (UserInterface|CreateWidget "/Game/GlobalGameJam/HUD/WBP_Victory.WBP_Victory_C"))
      (UserInterface|Viewport|AddtoViewport _returnvalue 0)
      (Game|SetGamePaused true)
      (Variables|/Script/Engine.PlayerController|SetbShowMouseCursor (Game|GetPlayerController 0) true))))

(event EventBeginPlay
  (bind _mesh (Variables|Character|GetMesh))
  ;[1 1 1] HUD
  (bind _returnvalue (UserInterface|CreateWidget "/Game/GlobalGameJam/HUD/WBP_Game.WBP_Game_C"))
  (Variables|Default|SetWBPGame _returnvalue)
  (UserInterface|Viewport|AddtoViewport _returnvalue 0)
  (Audio|PlaySoundatLocation "/Game/GlobalGameJam/Assets/Audio/DSRap.DSRap" "0, 0, 0" "0, 0, 0" 1.0 1.0 0.0 0 0 0)
  (Audio|PlaySoundatLocation "/Game/GlobalGameJam/Assets/Audio/D_S_Flute_track_5_2.D_S_Flute_track_5_2" "0, 0, 0" "0, 0, 0" 1.0 1.0 0.0 0 0 0)
  (switch int (Math|Random|RandomInteger 5)
    (:Default
      (Class|SkinnedMeshComponent|SetSkeletalMesh _mesh "/Game/GlobalGameJam/Assets/Models/Angry_T-Pose.Angry_T-Pose" true :!label _label)
      (Class|SkeletalMeshComponent|SetAnimClass _mesh "/Game/GlobalGameJam/Assets/Animations/A_Angry.A_Angry_C")
      (Class|NiagaraComponent|SetAsset (Variables|Default|GetFX_Constellation) "/Game/GlobalGameJam/Assets/VFX/FX_Angry.FX_Angry"))
    (:0
      (goto _label))
    (:1
      (Class|SkinnedMeshComponent|SetSkeletalMesh (Variables|Character|GetMesh) "/Game/GlobalGameJam/Assets/Models/Glossy_T-Pose.Glossy_T-Pose" true)
      (Class|SkeletalMeshComponent|SetAnimClass (Variables|Character|GetMesh) "/Game/GlobalGameJam/Assets/Animations/A_Glossy.A_Glossy_C")
      (Class|NiagaraComponent|SetAsset (Variables|Default|GetFX_Constellation) "/Game/GlobalGameJam/Assets/VFX/FX_Glossy.FX_Glossy"))
    (:2
      (Class|SkinnedMeshComponent|SetSkeletalMesh (Variables|Character|GetMesh) "/Game/GlobalGameJam/Assets/Models/Lanky_T-Pose.Lanky_T-Pose" true)
      (Class|SkeletalMeshComponent|SetAnimClass (Variables|Character|GetMesh) "/Game/GlobalGameJam/Assets/Animations/A_Lanky.A_Lanky_C")
      (Class|NiagaraComponent|SetAsset (Variables|Default|GetFX_Constellation) "/Game/GlobalGameJam/Assets/VFX/FX_Lanky.FX_Lanky"))
    (:3
      (Class|SkinnedMeshComponent|SetSkeletalMesh (Variables|Character|GetMesh) "/Game/GlobalGameJam/Assets/Models/Sticky_T-Pose.Sticky_T-Pose" true)
      (Class|SkeletalMeshComponent|SetAnimClass (Variables|Character|GetMesh) "/Game/GlobalGameJam/Assets/Animations/A_Sticky.A_Sticky_C")
      (Class|NiagaraComponent|SetAsset (Variables|Default|GetFX_Constellation) "/Game/GlobalGameJam/Assets/VFX/FX_Sticky.FX_Sticky"))
    (:4
      (Class|SkinnedMeshComponent|SetSkeletalMesh (Variables|Character|GetMesh) "/Game/GlobalGameJam/Assets/Models/Toddly_T-Pose.Toddly_T-Pose" true)
      (Class|SkeletalMeshComponent|SetAnimClass (Variables|Character|GetMesh) "/Game/GlobalGameJam/Assets/Animations/A_Toddly.A_Toddly_C")
      (Class|NiagaraComponent|SetAsset (Variables|Default|GetFX_Constellation) "/Game/GlobalGameJam/Assets/VFX/FX_Toddly.FX_Toddly"))))

(event Input|ActionEvents|InputActionDashForward
  (params (Key :type Key%20Structure :default "None"))
  (bind _returnvalue (Transformation|GetActorLocation))
  (bind _followcamera (Variables|Default|GetFollowCamera))
  (bind _followcamera_2 (Variables|Default|GetFollowCamera))
  (bind _speedwithboost (Variables|Default|GetSpeedWithBoost))
  (bind _speedwithoutboost (Variables|Default|GetSpeedWithoutBoost))
  (bind _volumewhoosh (Variables|Default|GetVolumeWhoosh))
  (bind _returnvalue_2 (Math|Vector|GetForwardVector _followcamera))
  (bind _returnvalue_3 (Math|Vector|GetForwardVector _followcamera_2))
  ;[1 1 1] Dash
  (:Pressed
    (if (not (Variables|Default|GetDashActivated))
      (Utilities|FlowControl|FlipFlop
        (:A
          (Audio|PlaySoundatLocation "/Game/GlobalGameJam/Assets/Audio/Whoosh/whoosh_high_1.whoosh_high_1" _returnvalue "0, 0, 0" _volumewhoosh 1.0 0.0 0 0 0))
        (:B
          (Audio|PlaySoundatLocation "/Game/GlobalGameJam/Assets/Audio/Whoosh/whoosh_mid_1.whoosh_mid_1" _returnvalue "0, 0, 0" _volumewhoosh 1.0 0.0 0 0 0)))
      (bind _returnvalue_4 (Class|GlobalGameJamCharacter|GetCanBoost))
      (if _returnvalue_4
        (CallFunction|Dash (* _returnvalue_3 _speedwithboost))
        (Variables|Default|SetLastSpeedValue _speedwithboost)
        (Variables|Default|SetLastDirection _returnvalue_3)
        (Variables|Default|SetDashActivated true)
        ;;[1 1 1] If the player click correctly
        (if (not (Variables|Default|GetBoostedActivated))
          (bind _output_get (Variables|Default|SetBeatAcumulated (+ (Variables|Default|GetBeatAcumulated) (Variables|Default|GetBeatCharged))))
          (if (>= _output_get 1.0)
            (Variables|Default|SetBoostedActivated true)
            (bind _beat (Timeline|BeatDecrease Play)
              (:Update
                (Variables|Default|SetBeatAcumulated _beat))
              (:Finished
                (Variables|Default|SetBoostedActivated false)))))
        (else
          (CallFunction|Dash (* _returnvalue_2 _speedwithoutboost))
          (Variables|Default|SetLastSpeedValue _speedwithoutboost)
          (Variables|Default|SetLastDirection _returnvalue_2)
          (Variables|Default|SetDashActivated true))))))

(event Input|ActionEvents|InputActionDashBack
  (params (Key :type Key%20Structure :default "None"))
  (bind _returnvalue (Transformation|GetActorLocation))
  (bind _followcamera (Variables|Default|GetFollowCamera))
  (bind _followcamera_2 (Variables|Default|GetFollowCamera))
  (bind _speedwithboost (Variables|Default|GetSpeedWithBoost))
  (bind _speedwithoutboost (Variables|Default|GetSpeedWithoutBoost))
  (bind _volumewhoosh (Variables|Default|GetVolumeWhoosh))
  (bind _returnvalue_2 (Math|Vector|GetForwardVector _followcamera))
  (bind _returnvalue_3 (Math|Vector|GetForwardVector _followcamera_2))
  (bind _returnvalue_4 (* _speedwithoutboost -1.0))
  (bind _returnvalue_5 (* _speedwithboost -1.0))
  ;[1 1 1] Dash
  (:Pressed
    (if (not (Variables|Default|GetDashActivated))
      (Utilities|FlowControl|FlipFlop
        (:A
          (Audio|PlaySoundatLocation "/Game/GlobalGameJam/Assets/Audio/Whoosh/whoosh_mid_2.whoosh_mid_2" _returnvalue "0, 0, 0" _volumewhoosh 1.0 0.0 0 0 0))
        (:B
          (Audio|PlaySoundatLocation "/Game/GlobalGameJam/Assets/Audio/Whoosh/whoosh_low_2_.whoosh_low_2_" _returnvalue "0, 0, 0" _volumewhoosh 1.0 0.0 0 0 0)))
      (bind _returnvalue_6 (Class|GlobalGameJamCharacter|GetCanBoost))
      (if _returnvalue_6
        (CallFunction|Dash (* _returnvalue_3 _returnvalue_5))
        (Variables|Default|SetLastSpeedValue _returnvalue_5)
        (Variables|Default|SetLastDirection _returnvalue_3)
        (Variables|Default|SetDashActivated true)
        ;;[1 1 1] If the player click correctly
        (if (not (Variables|Default|GetBoostedActivated))
          (bind _output_get (Variables|Default|SetBeatAcumulated (+ (Variables|Default|GetBeatAcumulated) (Variables|Default|GetBeatCharged))))
          (if (>= _output_get 1.0)
            (Variables|Default|SetBoostedActivated true)
            (bind _beat (Timeline|BeatDecrease Play)
              (:Update
                (Variables|Default|SetBeatAcumulated _beat))
              (:Finished
                (Variables|Default|SetBoostedActivated false)))))
        (else
          (CallFunction|Dash (* _returnvalue_2 _returnvalue_4))
          (Variables|Default|SetLastSpeedValue _returnvalue_4)
          (Variables|Default|SetLastDirection _returnvalue_2)
          (Variables|Default|SetDashActivated true))))))

(event Input|ActionEvents|InputActionPause
  (params (Key :type Key%20Structure :default "None"))
  ;[1 1 1] Pause
  (:Pressed
    (Game|SetGamePaused true)
    (bind _returnvalue (UserInterface|CreateWidget "/Game/GlobalGameJam/HUD/WBP_Victory.WBP_Victory_C"))
    (UserInterface|Viewport|AddtoViewport _returnvalue 0)
    (Variables|/Script/Engine.PlayerController|SetbShowMouseCursor (Game|GetPlayerController 0) true)))

(event Input|KeyboardEvents|Z
  (params (Key :type Key%20Structure :default "None"))
  (bind _returnvalue (Game|GetPlayerController 0))
  (bind _returnvalue_2 (Game|GetPlayerController 0))
  ;[1 1 1] Mouse Sensitivity
  (:Pressed
    (Utilities|FlowControl|FlipFlop
      (:A
        (bind _returnvalue_3 (UserInterface|CreateWidget "/Game/GlobalGameJam/Blueprints/Mouse_Sensitivity.Mouse_Sensitivity_C"))
        (UserInterface|Viewport|AddtoViewport _returnvalue_3 0)
        (Variables|/Script/Engine.PlayerController|SetbShowMouseCursor _returnvalue_2 true)
        (Input|SetInputModeGameandUI _returnvalue_2 _returnvalue_3 "LockAlways" false))
      (:B
        (Widget|RemovefromParent _returnvalue_3)
        (Variables|/Script/Engine.PlayerController|SetbShowMouseCursor _returnvalue false)
        (Class|WidgetBlueprintLibrary|SetFocustoGameViewport)
        (Input|SetInputModeGameOnly _returnvalue)))))

(event Input|KeyboardEvents|X
  (params (Key :type Key%20Structure :default "None"))
  (:Pressed
    (Development|PrintString (Utilities|String|ToString(Float) (Variables|Default|GetMouse%20Sensitivity)))))

(fn ConstructionScript)

(fn Dash
  (params (Velocity :type Vector))
  (Character|LaunchCharacter Velocity false false)
  (return))